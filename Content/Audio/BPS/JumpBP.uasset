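; An animation notify that plays a jump sound suited to the surface under the character.
; It line-traces 150 units down from the mesh, reads the hit's surface type and spawns the sound attached to the mesh.
; Rubber and Concrete each set an Index, but the sound's "Materials" integer parameter receives a constant zero instead of that Index.
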(fn `Received_Notify`
  (params (MeshComp :type "SkeletalMeshComponent Object Reference") (Animation :type "AnimSequenceBase Object Reference") (EventReference :type "AnimNotifyEventReference Structure (by ref)"))
  (returns (ReturnValue :type Boolean))
  (locals (Materials :type "EPhysicalSurface Enum") (FS :type "AudioComponent Object Reference") (Index :type Integer))
  (bind _returnvalue (`SceneComponent.K2_GetComponentLocation` MeshComp))
  (bind (_outhit _returnvalue_2) (`KismetSystemLibrary.LineTraceSingle` _returnvalue (- _returnvalue (0.0 0.0 150.0)) "TraceTypeQuery1"))
  (if _returnvalue_2
    (set `local.Materials` (`GameplayStatics.GetSurfaceType` _outhit))
    (bind _returnvalue_3 (`GameplayStatics.SpawnSoundAttached` "/Game/Audio/Movement/Soundcue/Jump.Jump" MeshComp (`self.Bone`) (0.0 0.0 0.0) (struct) "KeepRelativeOffset" false 1.0 1.0 0.0 null null))
    (set `local.FS` _returnvalue_3)
    (switch `EPhysicalSurface` (`local.Materials`)
      (:`SurfaceType1`
        (set `local.Index` 0))
      (:`SurfaceType2`
        (set `local.Index` 1)))
    (`AudioParameterControllerInterface.SetIntParameter` (`local.FS`) "Materials" 0)
    (return false)))